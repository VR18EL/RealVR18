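; BP_ScreamGrab is a grabbable object that screams while held and reacts to being hit by the umbrella weapon.
; Grab events from GrabComponent play the scream and start a looping timer that replays it, and dropping clears the timer.
; A mesh hit by BP_WeaponUm swaps the audio to SoundHuck and plays it.
; The scream sound is never restored, so later grab screams use SoundHuck.
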(event `self.ReceiveBeginPlay`
  (`AudioComponent.SetSound` (`self.Audio`) "/Game/DK/Sound/ScreamSound.ScreamSound"))

(event `self.GrabComponent.OnGrabbed`
  ;[1 1 1] Scream on Grabbed
  (`self.PlayScream`)
  (`KismetSystemLibrary.K2_SetTimer` null "PlayScream" 3.0 true))

(event `self.GrabComponent.OnDropped`
  ;[1 1 1] Stop Scream on Dropped
  (`KismetSystemLibrary.K2_ClearTimer` null "PlayScream"))

(event `self.ScreamStaticMesh.OnComponentHit`
  (params (HitComponent :type "PrimitiveComponent Object Reference") (OtherActor :type "Actor Object Reference") (OtherComp :type "PrimitiveComponent Object Reference") (NormalImpulse :type "Vector Structure") (Hit :type "HitResult Structure (by ref)"))
  ;[1 1 1] 우산에 맞았는가?
  (if (== (`GameplayStatics.GetObjectClass` OtherActor) "/Game/DK/Blueprints/BP_WeaponUm.BP_WeaponUm_C")
    ;[1 1 1] Set Audio after hit and Play
    (`AudioComponent.SetSound` (`self.Audio`) "/Game/DK/Sound/SoundHuck.SoundHuck")
    (`AudioComponent.Play` (`self.Audio`) 0.0)))

(fn `PlayScream`
  (`AudioComponent.Play` (`self.Audio`) 0.0))

(fn `UserConstructionScript`)